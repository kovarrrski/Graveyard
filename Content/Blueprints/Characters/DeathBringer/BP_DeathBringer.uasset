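; BP_DeathBringer is the DeathBringer character, a sprite-based pawn that moves along the world X axis.
; Every Tick updates facing, then feeds MovementDirection as the scale into movement input.
; Facing snaps the whole actor's rotation by the sign of MovementDirection, so zero gets the same flipped rotation as negative values.
; Nothing in this graph sets MovementDirection.
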(event `self.ReceiveTick`
  (params (DeltaSeconds :type "Float (single-precision)"))
  (`self.HandleRotation`)
  (`self.HandleMovement`))

(event `HandleMovement`
  (`self.AddMovementInput` (1.0 0.0 0.0) (`self.MovementDirection`)))

(event `HandleRotation`
  ;[1 1 1] Sprite Rotation depends on +- X of MovementDirection
  (if (> (`self.MovementDirection`) 0.0)
    (`self.K2_SetActorRotation` (struct))
    (else
      (`self.K2_SetActorRotation` (struct :`Yaw` 180.0)))))

(fn `UserConstructionScript`)